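; BP_Door is a key-locked door with an indicator light that reacts to the first-person player.
; BeginPlay caches the player and applies a dynamic material instance to the light mesh.
; Entering the collision volume brightens the light, turning it green and rotating the door open via a Timeline if HasKey is true, otherwise red.
; Leaving restores the dimmer amber light and reverses the Timeline.
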(event `self.ReceiveBeginPlay`
  ; Set up
  (bind _asbp_first_person_character (cast `/Game/StarterContent/FirstPerson/Blueprints/BP_FirstPersonCharacter` (`GameplayStatics.GetPlayerCharacter` 0)))
  (set `self.Player_Ref` _asbp_first_person_character)
  (bind _returnvalue (`KismetMaterialLibrary.CreateDynamicMaterialInstance` "/Game/MyContent/Materials/MI_Door_Light.MI_Door_Light"))
  (set `self.Dynamic Material` _returnvalue)
  (`PrimitiveComponent.SetMaterial` (`self.SM_Light`) 0 (`self.Dynamic Material`)))

(event `self.Collision.OnComponentBeginOverlap`
  (params (OverlappedComponent :type "PrimitiveComponent Object Reference") (OtherActor :type "Actor Object Reference") (OtherComp :type "PrimitiveComponent Object Reference") (OtherBodyIndex :type Integer) (bFromSweep :type Boolean) (SweepResult :type "HitResult Structure (by ref)"))
  (bind _dynamic_material (`self.Dynamic Material`))
  ; Light Change
  (if (== OtherActor (`self.Player_Ref`))
    (`MaterialInstanceDynamic.SetScalarParameterValue` _dynamic_material "Intensity" 100.0)
    (if (`/Game/StarterContent/FirstPerson/Blueprints/BP_FirstPersonCharacter.HasKey` (`self.Player_Ref`))
      (`MaterialInstanceDynamic.SetVectorParameterValue` _dynamic_material "Colour" (struct :`R` 0.070692 :`G` 1.0 :`A` 1.0))
      ; Door Animation
      (bind (_direction _alpha) (`Timeline|Timeline` :!label _label)
        (:`Update`
          (`SceneComponent.K2_SetRelativeRotation` (`self.SM_Door`) (`KismetMathLibrary.RLerp` (struct) (struct :`Yaw` 90.0) _alpha) false false)))
      (else
        (`MaterialInstanceDynamic.SetVectorParameterValue` _dynamic_material "Colour" (struct :`R` 1.0 :`B` 0.011649 :`A` 1.0))))))

(event `self.Collision.OnComponentEndOverlap`
  (params (OverlappedComponent :type "PrimitiveComponent Object Reference") (OtherActor :type "Actor Object Reference") (OtherComp :type "PrimitiveComponent Object Reference") (OtherBodyIndex :type Integer))
  (bind _dynamic_material (`self.Dynamic Material`))
  ; Light Default
  (if (== OtherActor (`self.Player_Ref`))
    (`MaterialInstanceDynamic.SetScalarParameterValue` _dynamic_material "Intensity" 1.0)
    (`MaterialInstanceDynamic.SetVectorParameterValue` _dynamic_material "Colour" (struct :`R` 1.0 :`G` 0.741098 :`B` 0.215883 :`A` 1.0))
    (goto _label :!via `Reverse`)))

(fn `UserConstructionScript`)