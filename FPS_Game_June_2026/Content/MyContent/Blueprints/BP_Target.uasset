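; BP_Target is a moving, destructible target actor that shuttles back and forth and takes a set number of hits.
; A looping timer reverses Direction every MovementDuration, while Tick offsets the actor along it by Speed per frame, unscaled by delta time and without sweep.
; Each Hit event decrements Hitpoints and spawns a particle effect and explosion sound at the hit location, with a bigger sound and actor destruction at zero.
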(event `self.ReceiveBeginPlay`
  ;[0.7468 0.295 0.7552 0.5] Flip Direction
  (`KismetSystemLibrary.K2_SetTimerDelegate` (delegate `Event FlipDirection`) (`self.MovementDuration`) true))

(event `Event FlipDirection`
  ;[0.7468 0.295 0.7552 0.5] Flip Direction
  (set `self.Direction` (* (`self.Direction`) -1.0)))

(event `self.ReceiveTick`
  (params (DeltaSeconds :type "Float (single-precision)"))
  ;[0.6979 0.3552 0.1613 0.5] Movement
  (`self.K2_AddActorWorldOffset` (* (`KismetMathLibrary.Normal` (`self.Direction`)) (`self.Speed`))))

(event `self.ReceiveHit`
  (params (MyComp :type "PrimitiveComponent Object Reference") (Other :type "Actor Object Reference") (OtherComp :type "PrimitiveComponent Object Reference") (bSelfMoved :type Boolean) (HitLocation :type "Vector Structure") (HitNormal :type "Vector Structure") (NormalImpulse :type "Vector Structure") (Hit :type "HitResult Structure (by ref)"))
  ; Target Destroy
  (set `self.Hitpoints` (- (`self.Hitpoints`) 1))
  (if (<= (`self.Hitpoints`) 0)
    (`NiagaraFunctionLibrary.SpawnSystemAtLocation` "/Game/MyContent/FX/PE_Target_Hit.PE_Target_Hit" HitLocation)
    (`GameplayStatics.SpawnSoundAtLocation` "/Game/MyContent/Audio/MP3_Explosion_Big.MP3_Explosion_Big" HitLocation (struct) 1.0 1.0 0.0 null null)
    (`self.K2_DestroyActor`)
    (else
      (`NiagaraFunctionLibrary.SpawnSystemAtLocation` "/Game/MyContent/FX/PE_Target_Hit.PE_Target_Hit" HitLocation)
      (`GameplayStatics.SpawnSoundAtLocation` "/Game/MyContent/Audio/MP3_Explosions_Small.MP3_Explosions_Small" HitLocation (struct) 1.0 1.0 0.0 null null))))

(fn `UserConstructionScript`)